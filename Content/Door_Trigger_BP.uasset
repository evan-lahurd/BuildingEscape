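; Blueprint that swings a referenced Door actor open and closed in response to OpenDoor's OnOpen and OnClose events.
; The DoorSwing timeline plays or reverses, combining its yaw curve with the door rotation cached at BeginPlay.
; An event track on the same timeline checks playback direction to play the open or close sound at the door's location.
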(event `self.ReceiveBeginPlay`
  (set `self.Initial Rotation` (`self.K2_GetActorRotation` (`self.Door`))))

(event `self.OpenDoor.OnOpen`
  (bind _returnvalue (`self.K2_GetActorLocation` (`self.Door`)))
  (bind (_direction _door_swing) (`Timeline|Door Swing` :!label _label)
    (:`Update`
      (`self.SetActorRotation` (`self.Door`) (`KismetMathLibrary.ComposeRotators` (`KismetMathLibrary.MakeRotator` 0.0 0.0 _door_swing) (`self.Initial Rotation`))))
    (:`Open Door Timing`
      (switch `ETimelineDirection` _direction
        (:`Forward`
          (`GameplayStatics.PlaySoundAtLocation` "/Game/Audio/Door_Open.Door_Open" _returnvalue))
        (:`Backward`
          (`GameplayStatics.PlaySoundAtLocation` "/Game/Audio/Door_Close.Door_Close" _returnvalue))))))

(event `self.OpenDoor.OnClose`
  (goto _label :!via `Reverse`))

(fn `UserConstructionScript`)